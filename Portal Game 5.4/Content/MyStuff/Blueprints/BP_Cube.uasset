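; BP_Cube is a portal projectile that places a blue or non-blue BP_Portal where it hits.
; On hit it destroys existing portals of the same color, spawns a new one aligned to the impact normal, then destroys itself.
; An angle check detects floor and ceiling hits, where portal yaw comes from the Arrow component instead of the normal.
; Hitting a PortalBlock component only prints a message and does not stop placement.
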(event OnComponentHit(Cube)
  (params (HitComponent :type Primitive%20Component%20Object%20Reference) (OtherActor :type Actor%20Object%20Reference) (OtherComp :type Primitive%20Component%20Object%20Reference) (NormalImpulse :type Vector :default "0, 0, 0") (Hit :type Hit%20Result%20Structure%20%28by%20ref%29))
  (if (== (Variables|Default|GetPortalBlock) OtherComp)
    (Development|PrintString "Portal Block"))
  (bind _outactors (Actor|GetAllActorsOfClass "/Game/MyStuff/Blueprints/BP_Portal.BP_Portal_C"))
  (for _array_element _outactors
    (if (== (Variables|/Game/MyStuff/Blueprints/BP_Portal.BP_Portal_C|GetisBlueportal _array_element) (Variables|Default|GetisBlueProjectile))
      (Actor|DestroyActor _array_element)))
  (CallFunction|RotateForward))

(event Custom|RotateForward
  (bind _angle (CallFunction|AngleBetweenTwoVectors (Math|Vector|Normalize (.normal (stale OnComponentHit(Cube) Hit))) "0.000000,0.000000,1.000000"))
  (if (< _angle 1.0)
    (bind _returnvalue (Game|SpawnActorfromClass "/Game/MyStuff/Blueprints/BP_Portal.BP_Portal_C" (Math|Transform|MakeTransform (.impactpoint (stale OnComponentHit(Cube) Hit)) (Math|Rotator|MakeRotator (.roll (Math|Conversions|RotationFromXVector (.normal (stale OnComponentHit(Cube) Hit)))) (.pitch (Math|Conversions|RotationFromXVector (.normal (stale OnComponentHit(Cube) Hit)))) (.yaw (Transformation|GetWorldRotation (Variables|Default|GetArrow)))) "1.000000,1.000000,1.000000") "Undefined" "MultiplyWithRoot" 0 0 :!label _label))
    (Variables|/Game/MyStuff/Blueprints/BP_Portal.BP_Portal_C|SetisBlueportal _returnvalue (Variables|Default|GetisBlueProjectile))
    (Actor|DestroyActor)
    (else
      (bind _angle_2 (CallFunction|AngleBetweenTwoVectors (Math|Vector|Normalize (.normal (stale OnComponentHit(Cube) Hit))) "0.000000,0.000000,-1.000000"))
      (if (< _angle_2 1.0)
        (goto _label)
        (else
          (bind _returnvalue_2 (Game|SpawnActorfromClass "/Game/MyStuff/Blueprints/BP_Portal.BP_Portal_C" (Math|Transform|MakeTransform (.impactpoint (stale OnComponentHit(Cube) Hit)) (Math|Rotator|MakeRotator (.roll (Math|Conversions|RotationFromXVector (.normal (stale OnComponentHit(Cube) Hit)))) (.pitch (Math|Conversions|RotationFromXVector (.normal (stale OnComponentHit(Cube) Hit)))) (.yaw (Math|Conversions|RotationFromXVector (.normal (stale OnComponentHit(Cube) Hit))))) "1.000000,1.000000,1.000000") "Undefined" "MultiplyWithRoot" 0 0))
          (Variables|/Game/MyStuff/Blueprints/BP_Portal.BP_Portal_C|SetisBlueportal _returnvalue_2 (Variables|Default|GetisBlueProjectile))
          (Actor|DestroyActor))))))

(event EventBeginPlay
  (bind _returnvalue (Actor|GetActorOfClass "/Game/FirstPerson/Blueprints/BP_FirstPersonCharacter.BP_FirstPersonCharacter_C"))
  (Variables|Default|SetPlayer _returnvalue))

(fn ConstructionScript)

(fn AngleBetweenTwoVectors
  (params (Vector%20A :type Vector) (Vector%20B :type Vector))
  (return (Class|KismetMathLibrary|DegAcos (Math|Vector|DotProduct (Math|Vector|Normalize Vector%20A) (Math|Vector|Normalize Vector%20B)))))