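; BP_Door is a sliding door that opens when the first-person character overlaps it and closes when they leave, unless IsButtonActivated is set.
; OpenDoor and CloseDoor events toggle a DoorIsOpen flag, so a button-activated door relies on those events being called from outside this graph.
; Tick moves the Door component along its relative Y axis at DoorSpeed, clamping the offset between closed and DoorMaxOffset.
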(event Custom|CloseDoor
  (Variables|Default|SetDoorIsOpen false))

(event Custom|OpenDoor
  (Variables|Default|SetDoorIsOpen true))

(event Collision|EventActorBeginOverlap
  (params (OtherActor :type Actor%20Object%20Reference))
  (Utilities|Casting|CastToBP_FirstPersonCharacter OtherActor)
  (if (not (Variables|Default|GetIsButtonActivated))
    (CallFunction|OpenDoor)))

(event EventTick
  (params (DeltaSeconds :type Float%20%28single-precision%29))
  (bind _door (Variables|Default|GetDoor))
  (bind _door_2 (Variables|Default|GetDoor))
  (bind _relativelocation (Variables|/Script/Engine.SceneComponent|GetRelativeLocation _door))
  (bind _relativelocation_2 (Variables|/Script/Engine.SceneComponent|GetRelativeLocation _door_2))
  (if (Variables|Default|GetDoorIsOpen)
    (bind _output_get (Variables|Default|SetDoorOffset (Math|Float|Clamp(Float) (+ (* DeltaSeconds (Variables|Default|GetDoorSpeed)) (Variables|Default|GetDoorOffset)) 0.0 (Variables|Default|GetDoorMaxOffset))))
    (Transformation|SetRelativeLocation _door_2 (Math|Vector|MakeVector (.x _relativelocation_2) _output_get (.z _relativelocation_2)) false false)
    (else
      (bind _output_get_2 (Variables|Default|SetDoorOffset (Math|Float|Clamp(Float) (- (Variables|Default|GetDoorOffset) (* DeltaSeconds (Variables|Default|GetDoorSpeed))) 0.0 (Variables|Default|GetDoorMaxOffset))))
      (Transformation|SetRelativeLocation _door (Math|Vector|MakeVector (.x _relativelocation) _output_get_2 (.z _relativelocation)) false false))))

(event Collision|EventActorEndOverlap
  (params (OtherActor :type Actor%20Object%20Reference))
  (Utilities|Casting|CastToBP_FirstPersonCharacter OtherActor)
  (if (not (Variables|Default|GetIsButtonActivated))
    (CallFunction|CloseDoor)))

(fn ConstructionScript)