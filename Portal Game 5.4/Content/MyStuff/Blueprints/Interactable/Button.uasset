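; Interactable button actor that toggles a linked door open and closed.
; On BeginPlay it sets its mesh material to the on or off look from the IsActivated flag, without moving the door.
; Each Interact call flips the flag, swaps the material and calls OpenDoor or CloseDoor on the referenced DoorActor.
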(event EventBeginPlay
  (if (Variables|Default|GetIsActivated)
    (Rendering|Material|SetMaterial (Variables|Default|Get%20Button) 0 "/Game/MyStuff/Materials/MI_ButtonOn.MI_ButtonOn")
    (else
      (Rendering|Material|SetMaterial (Variables|Default|Get%20Button) 0 "/Game/MyStuff/Materials/MI_ButtonOff.MI_ButtonOff"))))

(event Collision|EventActorBeginOverlap
  (params (OtherActor :type Actor%20Object%20Reference)))

(event EventTick
  (params (DeltaSeconds :type Float%20%28single-precision%29)))

(event EventInteract
  (bind _dooractor (Variables|Default|GetDoorActor))
  (if (Variables|Default|GetIsActivated)
    (Variables|Default|SetIsActivated false)
    (Rendering|Material|SetMaterial (Variables|Default|Get%20Button) 0 "/Game/MyStuff/Materials/MI_ButtonOff.MI_ButtonOff")
    (Default|CloseDoor _dooractor)
    (else
      (Variables|Default|SetIsActivated true)
      (Rendering|Material|SetMaterial (Variables|Default|Get%20Button) 0 "/Game/MyStuff/Materials/MI_ButtonOn.MI_ButtonOn")
      (Default|OpenDoor _dooractor))))

(fn ConstructionScript)