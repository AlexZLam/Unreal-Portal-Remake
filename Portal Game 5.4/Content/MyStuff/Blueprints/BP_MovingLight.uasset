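; BP_MovingLight is an actor whose point light slides along its local Y axis when the first-person character overlaps it.
; Overlap calls MoveLight to set a movement flag, while StopLight clears it but is not called within this Blueprint.
; Tick raises or lowers the offset by that flag at a frame-rate-independent speed, clamped between zero and a maximum, and applies it to the light's relative location.
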(event Custom|MoveLight
  (Variables|Default|SetLightMove true))

(event Custom|StopLight
  (Variables|Default|SetLightMove false))

(event Collision|EventActorBeginOverlap
  (params (OtherActor :type Actor%20Object%20Reference))
  (Utilities|Casting|CastToBP_FirstPersonCharacter OtherActor)
  (CallFunction|MoveLight))

(event EventTick
  (params (DeltaSeconds :type Float%20%28single-precision%29))
  (bind _pointlight (Variables|Default|GetPointLight))
  (bind _pointlight_2 (Variables|Default|GetPointLight))
  (bind _relativelocation (Variables|/Script/Engine.SceneComponent|GetRelativeLocation _pointlight_2))
  (bind _relativelocation_2 (Variables|/Script/Engine.SceneComponent|GetRelativeLocation _pointlight))
  (if (Variables|Default|GetLightMove)
    (bind _output_get (Variables|Default|SetLightOffset (Math|Float|Clamp(Float) (+ (* DeltaSeconds (Variables|Default|GetLightSpeed)) (Variables|Default|GetLightOffset)) 0.0 (Variables|Default|GetLightMaxOffset))))
    (Transformation|SetRelativeLocation _pointlight (Math|Vector|MakeVector (.x _relativelocation_2) _output_get (.z _relativelocation_2)) false false)
    (else
      (bind _output_get_2 (Variables|Default|SetLightOffset (Math|Float|Clamp(Float) (- (Variables|Default|GetLightOffset) (* DeltaSeconds (Variables|Default|GetLightSpeed))) 0.0 (Variables|Default|GetLightMaxOffset))))
      (Transformation|SetRelativeLocation _pointlight_2 (Math|Vector|MakeVector (.x _relativelocation) _output_get_2 (.z _relativelocation)) false false))))

(fn ConstructionScript)